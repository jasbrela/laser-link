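; BP_Mirror is a mirror actor that reflects a cannon's laser along the surface reflection vector, keeping its color.
; ReflectLaser reuses the previous iteration's beam at that index if this mirror owns it, otherwise takes a pooled beam or spawns a BP_LaserBeam.
; At the reflection limit it notifies the cannon that the laser has ended.
; ClearReflection deactivates the mirror's own beams and returns them to the available pool.
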(fn `CalculateTraceEnd`
  (params (`Trace Start` :type "Vector Structure") (Direction :type "Vector Structure") (SurfaceNormal :type "Vector Structure"))
  (returns (`Trace End` :type "Vector Structure"))
  (return (+ `Trace Start` (* (`KismetMathLibrary.GetReflectionVector` Direction SurfaceNormal) (`/Game/Blueprints/BPFL_Constants.GetLaserMaxLength`)))))

(fn `ClearReflection`
  (params (Laser :type "/Game/Blueprints/BP_LaserBeam Object Reference"))
  (`/Game/Blueprints/BP_MacroLibrary.Print` "Laser Deactivated." (struct :`R` 0.458824 :`B` 0.003922 :`A` 1.0))
  (if (`KismetArrayLibrary.Array_Contains` (`self.LaserBeamPool`) Laser)
    (`KismetArrayLibrary.Array_AddUnique` (`self.AvailableLaserBeams`) Laser)
    (`/Game/Blueprints/BP_LaserBeam.DeactivateLaser` Laser)
    (else
      (`/Game/Blueprints/BP_MacroLibrary.Print` "[BP_Mirror ClearReflection] Error" (struct :`R` 1.0 :`B` 0.007843 :`A` 1.0)))))

(fn `GetLaserFromAvailable`
  (params (RemoveFromAvailable :type Boolean))
  (returns (Laser :type "/Game/Blueprints/BP_LaserBeam Object Reference"))
  (locals (Temp :type "/Game/Blueprints/BP_LaserBeam Object Reference"))
  (bind _availablelaserbeams (`self.AvailableLaserBeams`))
  (bind _temp (`local.Temp`))
  (set `local.Temp` (`|GetArrayItem` _availablelaserbeams))
  (if RemoveFromAvailable
    (`KismetArrayLibrary.Array_RemoveItem` _availablelaserbeams _temp))
  (return _temp))

(fn `Reflect Laser`
  (params (Start :type "Vector Structure") (Direction :type "Vector Structure") (`Surface Normal` :type "Vector Structure") (Color :type "LinearColor Structure") (Cannon :type "/Game/Blueprints/BP_LaserCannon Object Reference") (`Previous Reflections` :type "Array of /Game/Blueprints/BP_LaserBeam Object Reference") (`Current Reflections` :type "Array of /Game/Blueprints/BP_LaserBeam Object Reference"))
  (locals (`Trace End` :type "Vector Structure" :default (0.0 0.0 0.0)) (`Trace Start` :type "Vector Structure") (_Color :type "LinearColor Structure") (_Cannon :type "/Game/Blueprints/BP_LaserCannon Object Reference") (_Laser :type "/Game/Blueprints/BP_LaserBeam Object Reference"))
  (bind _output (`|GetArrayItem` (`self.PreviousReflections`) (`KismetArrayLibrary.Array_Length` (`self.CurrentReflections`))))
  (`KismetSystemLibrary.PrintString` (`KismetStringLibrary.Concat_StrStr` "REFLECT: " (`KismetSystemLibrary.GetDisplayName` self)))
  (if (< (`KismetArrayLibrary.Array_Length` `Current Reflections`) (`/Game/Blueprints/BPFL_Constants.GetMaxReflections`))
    (`self.InitializeVariables` Start Direction `Surface Normal` Color Cannon `Previous Reflections` `Current Reflections`)
    (`self.IsOwner`
      (:`Is Owner`
        (`self.ShootLaserFromCurrentData` _output)
        (`self.SafeCheck` _output))
      (:`Not Owner`
        (`self.IsAnyLaserAvailable`
          (:`Available`
            (bind _laser (`self.GetLaserFromAvailable` true))
            (set `local._Laser` _laser))
          (:`Not available`
            (bind _laser_2 (`self.SpawnLaser`))
            (set `local._Laser` _laser_2)))
        (`self.ShootLaserFromCurrentData` (`local._Laser`))))
    (else
      (`/Game/Blueprints/BP_LaserCannon.ReachedEndOfLaser` Cannon `Current Reflections` `Previous Reflections`))))

(fn `UserConstructionScript`)