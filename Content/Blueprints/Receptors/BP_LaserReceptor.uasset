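; Laser receptor puzzle target that lights up when hit by a cannon with a matching ID, with one enum ID accepting any cannon.
; It tracks the cannons reaching it, deactivating when the last leaves or a mismatched one is the only hit.
; State changes swap four cylinder materials, toggle connect/disconnect sounds or effects and notify BP_GameMode of completion or failure.
; Successful hits are also reported back to the cannon.
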(event `self.ReceiveBeginPlay`)

(fn `ChangeMaterial`
  (params (Material :type "MaterialInterface Object Reference"))
  (`PrimitiveComponent.SetMaterial` (`self.Cylinder1`) 0 Material)
  (`PrimitiveComponent.SetMaterial` (`self.Cylinder2`) 0 Material)
  (`PrimitiveComponent.SetMaterial` (`self.Cylinder3`) 0 Material)
  (`PrimitiveComponent.SetMaterial` (`self.Cylinder4`) 0 Material))

(fn `NegativeFeedback`
  (if (`self.IsActive`)
    (`self.ChangeMaterial` "/Game/Material/M_NegativeLight.M_NegativeLight")
    (set `self.IsActive` false)
    (`AudioComponent.Stop` (`self.laser_connected`))
    (`AudioComponent.Play` (`self.laser_disconnected`) 0.0)
    (bind _asbp_game_mode (cast `/Game/Blueprints/BP_GameMode` (`GameplayStatics.GetGameMode`)))
    (`/Game/Blueprints/BP_GameMode.OnReceptorFailed` _asbp_game_mode)))

(fn `PositiveFeedback`
  (if (not (`self.IsActive`))
    (set `self.IsActive` true)
    (`AudioComponent.Stop` (`self.laser_disconnected`))
    (`AudioComponent.Play` (`self.laser_connected`) 0.0)
    (`self.ChangeMaterial` "/Game/Material/M_PositiveLight.M_PositiveLight")
    (bind _asbp_game_mode (cast `/Game/Blueprints/BP_GameMode` (`GameplayStatics.GetGameMode`)))
    (`/Game/Blueprints/BP_GameMode.OnReceptorCompleted` _asbp_game_mode)))

(fn `ReachReceptor`
  (params (Cannon :type "/Game/Blueprints/BP_LaserCannon Object Reference"))
  (`KismetArrayLibrary.Array_AddUnique` (`self.Cannons`) Cannon)
  (if (or (`|EnumEquality` (`/Game/Blueprints/BP_LaserCannon.GetID` Cannon) (`self.ID`)) (`|EnumEquality` (`self.ID`) "NewEnumerator3"))
    (`self.PositiveFeedback`)
    (`/Game/Blueprints/BP_LaserCannon.Successfuly Reached Receptor` Cannon self)
    (elif (== (`KismetArrayLibrary.Array_Length` (`self.Cannons`)) 1)
      (`self.NegativeFeedback`))))

(fn `RegisterCannonNotReachingAnymore`
  (params (Cannon :type "/Game/Blueprints/BP_LaserCannon Object Reference"))
  (bind _cannons (`self.Cannons`))
  (`KismetArrayLibrary.Array_RemoveItem` _cannons Cannon)
  (if (== (`KismetArrayLibrary.Array_Length` _cannons) 0)
    (`self.NegativeFeedback`)))

(fn `UserConstructionScript`)