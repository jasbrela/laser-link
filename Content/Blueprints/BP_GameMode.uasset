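; BP_GameMode is the game mode that tracks progress on laser receptors and shows it on screen.
; On BeginPlay it creates the WBP_UI widget, gathers every BP_LaserReceptor in the level and passes the total to the widget as the maximum.
; Its OnReceptorCompleted and OnReceptorFailed events raise or lower the running count and push the new value to the widget.
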(event `self.ReceiveBeginPlay`
  ;[1 1 1] BeginPlay
  (bind _returnvalue (`|CreateWidget` "/Game/Blueprints/WBP_UI.WBP_UI_C"))
  (bind _output_get (set `self.ReceptorsUI` _returnvalue))
  (`UserWidget.AddToViewport` _output_get 0)
  (bind _outactors (`GameplayStatics.GetAllActorsOfClass` "/Game/Blueprints/BP_LaserReceptor.BP_LaserReceptor_C"))
  (bind _output_get_2 (set `self.AllReceptors` _outactors))
  (`/Game/Blueprints/WBP_UI.SetMaxReceptors` (`self.ReceptorsUI`) (`KismetArrayLibrary.Array_Length` _output_get_2)))

(event `OnReceptorCompleted`
  (bind _result (`/Engine/EditorBlueprintResources/StandardMacros.IncrementInt` (`self.ReceptorsCount`))
    (:`  `
      (`/Game/Blueprints/WBP_UI.UpdateReceptorsCount` (`self.ReceptorsUI`) _result))))

(event `OnReceptorFailed`
  (bind _result (`/Engine/EditorBlueprintResources/StandardMacros.DecrementInt` (`self.ReceptorsCount`))
    (:`  `
      (`/Game/Blueprints/WBP_UI.UpdateReceptorsCount` (`self.ReceptorsUI`) _result))))

(fn `UserConstructionScript`)