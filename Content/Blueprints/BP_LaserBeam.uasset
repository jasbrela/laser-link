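; BP_LaserBeam is one laser segment in a cannon, mirror and receptor system, fired through EShootLaser and throttled by a looping timer.
; Each shot line-traces, spawns a colored Niagara beam, and stretches a capsule along it for brief query collision.
; Mirror hits trigger reflection, receptor hits notify the receptor and origin cannon, and misses report ReceptorNotFound.
; Overlaps with other beams only print whether their cannon LaserIDs match.
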(event `self.ReceiveBeginPlay`
  (`KismetSystemLibrary.K2_SetTimer` null "HandleShoot" 0.05 true))

(event `self.ReceiveActorBeginOverlap`
  (params (OtherActor :type "Actor Object Reference"))
  (if true
    (bind _asbp_laser_beam (cast `/Game/Blueprints/BP_LaserBeam` OtherActor))
    (bind _cannon (`self.GetCannon` _asbp_laser_beam))
    (if (`|EnumEquality` (`/Game/Blueprints/BP_LaserCannon.LaserID` _cannon) (`/Game/Blueprints/BP_LaserCannon.LaserID` (`self.CannonOrigin`)))
      (`KismetSystemLibrary.PrintString` "Hit same laser")
      (else
        (`KismetSystemLibrary.PrintString` "Hit different laser" true true (struct :`R` 1.0 :`B` 0.10567 :`A` 1.0))))))

(event `self.ReceiveTick`
  (params (DeltaSeconds :type "Float (single-precision)")))

(event `EShootLaser`
  (params (Start :type "Vector Structure") (End :type "Vector Structure") (`Laser Color` :type "LinearColor Structure") (Cannon :type "/Game/Blueprints/BP_LaserCannon Object Reference"))
  (bind _last_hit_actor (`self.Last Hit Actor`))
  (bind _returnvalue (select `bool` (`self.Hit`) :`false` (`self.Trace End`) :`true` (`self.HitLocation`)))
  (`PrimitiveComponent.SetCollisionEnabled` (`self.Capsule`) "QueryOnly")
  (`self.Can Shoot`
    (:`then`
      (bind (_tracestart _traceend _lasercolor) (`self.SetInitialVariables` Start End `Laser Color` Cannon))
      (bind (_outhit _returnvalue_2) (`KismetSystemLibrary.LineTraceSingle` :`Start` _tracestart :`End` _traceend :`TraceChannel` "TraceTypeQuery1" :`TraceColor` _lasercolor :`DrawTime` 1.0))
      (bind (_bblockinghit _binitialoverlap _time _distance _location _impactpoint _normal _impactnormal _physmat _hitactor) (`GameplayStatics.BreakHitResult` _outhit))
      (`self.SetLinetraceVariables` _returnvalue_2 _location _hitactor _normal)
      (bind _returnvalue_3 (`NiagaraFunctionLibrary.SpawnSystemAtLocation` "/Game/FX/NS_Laser.NS_Laser" (`self.Trace Start`)))
      (`FXSystemComponent.SetColorParameter` _returnvalue_3 "Color" (`self.Laser Color`))
      (`FXSystemComponent.SetVectorParameter` _returnvalue_3 "LaserEnd" _returnvalue)
      (`self.SetCollisionPosition` (`KismetMathLibrary.VLerp` (`self.Trace Start`) _returnvalue 0.5))
      (if (`self.Hit`)
        (`self.SetCollisionSizeAndRotation` (`self.Trace Start`) (`self.HitLocation`))
        (bind _asbp_mirror (cast `/Game/Blueprints/BP_Mirror` _last_hit_actor)
          (:`then`
            (`/Game/Blueprints/BP_Mirror.Reflect Laser` _asbp_mirror (`self.HitLocation`) (`KismetMathLibrary.GetDirectionUnitVector` (`self.Trace Start`) (`self.Trace End`)) (`self.HitNormal`) (`self.Laser Color`) (`self.CannonOrigin`)))
          (:`CastFailed`
            (bind _asbp_laser_receptor (cast `/Game/Blueprints/BP_LaserReceptor` _last_hit_actor))
            (`/Game/Blueprints/BP_LaserReceptor.PositiveFeedback` _asbp_laser_receptor)
            (`/Game/Blueprints/BP_LaserCannon.ReachReceptor` (`self.CannonOrigin`) _asbp_laser_receptor)))
        (else
          (`/Game/Blueprints/BP_LaserCannon.ReceptorNotFound` (`self.CannonOrigin`))
          (`self.SetCollisionSizeAndRotation` (`self.Trace Start`) (`self.Trace End`))))
      (`KismetSystemLibrary.Delay` 0.05)
      (`PrimitiveComponent.SetCollisionEnabled` (`self.Capsule`) "NoCollision"))))

(fn `GetCannon`
  (returns (Cannon :type "/Game/Blueprints/BP_LaserCannon Object Reference"))
  (return (`self.CannonOrigin`)))

(fn `HandleShoot`
  (if (not (`self.CanShoot`))
    (set `self.CanShoot` true)))

(fn `SetCollisionPosition`
  (params (Position :type "Vector Structure"))
  (`SceneComponent.K2_SetWorldLocation` (`self.Capsule`) Position false false))

(fn `SetCollisionSizeAndRotation`
  (params (`Start Point` :type "Vector Structure") (`End Point` :type "Vector Structure"))
  (bind _capsule (`self.Capsule`))
  (`CapsuleComponent.SetCapsuleHalfHeight` _capsule (- (/ (`KismetMathLibrary.Vector_Distance` `Start Point` `End Point`) 2.0) 50.0) true)
  (`SceneComponent.K2_SetWorldRotation` _capsule (`KismetMathLibrary.FindLookAtRotation` (`SceneComponent.K2_GetComponentLocation` _capsule) `End Point`) false false)
  (`SceneComponent.K2_AddLocalRotation` _capsule (struct :`Yaw` 90.0 :`Roll` 90.0) false false))

(fn `UserConstructionScript`)