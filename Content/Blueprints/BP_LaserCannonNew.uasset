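; BP_LaserCannonNew is a laser cannon that fires a colored, reflectable beam and drives feedback on receptors.
; It spawns a BP_LaserBeam on BeginPlay, then re-fires it every Tick along the Arrow, passing itself and previous and current reflection lists.
; Callback functions give the hit receptor positive feedback, send negative feedback when none is found, and save each pass's reflections as the previous list.
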(event `self.ReceiveBeginPlay`
  (bind _returnvalue (`|SpawnActorFromClass` "/Game/Blueprints/BP_LaserBeam.BP_LaserBeam_C" (`KismetMathLibrary.MakeTransform` (`SceneComponent.K2_GetComponentLocation` (`self.Arrow`))) "Undefined" "MultiplyWithRoot" null null))
  (set `self.LaserBeam` _returnvalue))

(event `self.ReceiveTick`
  (params (DeltaSeconds :type "Float (single-precision)"))
  (bind _laserbeam (`self.LaserBeam`))
  (bind _currentreflections (`self.CurrentReflections`))
  (bind _returnvalue (`SceneComponent.K2_GetComponentLocation` (`self.Arrow`)))
  (`KismetArrayLibrary.Array_Clear` (`self.CurrentReflections`))
  (`KismetArrayLibrary.Array_AddUnique` _currentreflections _laserbeam)
  (`/Game/Blueprints/BP_LaserBeam.EShootLaser` _laserbeam _returnvalue (+ _returnvalue (* (`KismetMathLibrary.GetForwardVector` (`SceneComponent.K2_GetComponentRotation` (`self.Arrow`))) (`/Game/Blueprints/BPFL_Constants.GetLaserMaxLength`))) (`self.Color`) self (`self.PreviousReflections`) _currentreflections))

(fn `GetID`
  (returns (ID :type "/Game/Blueprints/E_LaserIDs Enum"))
  (return (`self.LaserID`)))

(fn `ReachedEndOfLaser`
  (params (CurrentReflections :type "Array of /Game/Blueprints/BP_LaserBeam Object Reference"))
  (set `self.PreviousReflections` CurrentReflections)
  (`KismetSystemLibrary.PrintString` "--- END OF ITERATION ---" true true (struct :`R` 0.634339 :`G` 0.228885 :`B` 1.0 :`A` 1.0))
  (return))

(fn `ReachReceptor`
  (params (Receptor :type "/Game/Blueprints/BP_LaserReceptor Object Reference"))
  (bind _output_get (set `self.LastHitReceptor` Receptor))
  (`/Game/Blueprints/BP_LaserReceptor.PositiveFeedback` _output_get))

(fn `ReceptorNotFound`
  (bind _lasthitreceptor (`self.LastHitReceptor`))
  (if (`KismetSystemLibrary.IsValid` _lasthitreceptor)
    (`/Game/Blueprints/BP_LaserReceptor.Negative Feedback` _lasthitreceptor)
    (set `self.LastHitReceptor` null)))

(fn `UserConstructionScript`)