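; BP_LaserCollision is a capsule-based collision actor for a laser that can be sized and aimed.
; SetScale sets the capsule half-height to half a given length minus a fixed margin.
; SetRotation turns the actor toward a target point, then adds a local quarter-turn.
; On overlap with another BP_LaserCollision whose origin is very close to its own, it only prints a hit message.
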(event `self.ReceiveActorBeginOverlap`
  (params (OtherActor :type "Actor Object Reference"))
  (if (<= (`KismetMathLibrary.Vector_Distance` (`self.K2_GetActorLocation` OtherActor) (`self.K2_GetActorLocation`)) 5.0)
    (cast `/Game/Blueprints/BP_LaserCollision` OtherActor)
    (`KismetSystemLibrary.PrintString` "LaserHit")))

(fn `SetRotation`
  (params (LookAt :type "Vector Structure"))
  (`self.K2_SetActorRotation` (`KismetMathLibrary.FindLookAtRotation` (`self.K2_GetActorLocation`) LookAt))
  (`self.K2_AddActorLocalRotation` (struct :`Yaw` 90.0)))

(fn `SetScale`
  (params (Length :type "Float (double-precision)"))
  (`CapsuleComponent.SetCapsuleHalfHeight` (`self.Capsule`) (- (/ Length 2.0) 100.0) true))

(fn `UserConstructionScript`)