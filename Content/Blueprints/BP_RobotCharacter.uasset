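; Robot character Blueprint that the player moves with Enhanced Input and uses to grab and release mirrors.
; On possession by BP_RobotController it adds the robot mapping context; movement follows control yaw.
; The grab input toggles between attaching whatever actor a forward Visibility trace hits, without a mirror check, and detaching all attached actors.
; Tick also sets a target location just ahead of the capsule, separate from the attachment logic.
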(event `EnhancedInput|/Game/Inputs/Mappings/RobotGrabMirror`
  (params (ActionValue :type Boolean) (ElapsedSeconds :type "Float (double-precision)") (TriggeredSeconds :type "Float (double-precision)") (InputAction :type "InputAction Object Reference" :default "/Game/Inputs/Mappings/RobotGrabMirror.RobotGrabMirror"))
  (bind _capsulecomponent (`self.CapsuleComponent`))
  (bind _returnvalue (`SceneComponent.K2_GetComponentLocation` _capsulecomponent))
  ;[1 1 1] Grabbing Mirror
  (:`Started`
    (if (`self.isGrabbingMirror`)
      (`self.K2_DetachFromActor` (`self.GetAttachedActors` true) "KeepWorld" "KeepWorld" "KeepWorld")
      (set `self.isGrabbingMirror` false)
      (`KismetSystemLibrary.PrintString` "Mirror Released")
      (else
        (bind _outhit (`KismetSystemLibrary.LineTraceSingle` _returnvalue (+ _returnvalue (* (`KismetMathLibrary.GetForwardVector` (`SceneComponent.K2_GetComponentRotation` _capsulecomponent)) 400.0)) "TraceTypeQuery1"))
        (bind (_bblockinghit _binitialoverlap _time _distance _location _impactpoint _normal _impactnormal _physmat _hitactor) (`GameplayStatics.BreakHitResult` _outhit))
        (if _bblockinghit
          (`self.K2_AttachToActor` _hitactor self "None" "KeepWorld" "KeepRelative" "KeepWorld" true)
          (set `self.isGrabbingMirror` true)
          (`KismetSystemLibrary.PrintString` "Mirror Grabbed")
          (else
            (`KismetSystemLibrary.PrintString` "No Mirror to Grab")))))))

(event `self.ReceiveTick` :!enabledstate Disabled
  (params (DeltaSeconds :type "Float (single-precision)"))
  (bind _capsulecomponent (`self.CapsuleComponent`))
  (if true
    (`PhysicsHandleComponent.SetTargetLocation` (+ (`SceneComponent.K2_GetComponentLocation` _capsulecomponent) (* (`KismetMathLibrary.GetForwardVector` (`SceneComponent.K2_GetComponentRotation` _capsulecomponent)) 100.0)))))

(event `EnhancedInput|/Game/Inputs/Mappings/RobotMove`
  (params (ActionValue :type "Vector2D Structure") (ElapsedSeconds :type "Float (double-precision)") (TriggeredSeconds :type "Float (double-precision)") (InputAction :type "InputAction Object Reference" :default "/Game/Inputs/Mappings/RobotMove.RobotMove"))
  (bind (_returnvalue_roll _returnvalue_pitch _returnvalue_yaw) (`KismetMathLibrary.BreakRotator` (`self.GetControlRotation`)))
  (bind (_returnvalue_roll_2 _returnvalue_pitch_2 _returnvalue_yaw_2) (`KismetMathLibrary.BreakRotator` (`self.GetControlRotation`)))
  ;[1 1 1] Movement
  (:`Triggered`
    (`self.AddMovementInput` (`KismetMathLibrary.GetRightVector` (`KismetMathLibrary.MakeRotator` _returnvalue_roll 0.0 _returnvalue_yaw)) ActionValue_X)
    (`self.AddMovementInput` (`KismetMathLibrary.GetForwardVector` (`KismetMathLibrary.MakeRotator` 0.0 0.0 _returnvalue_yaw_2)) ActionValue_Y)))

(event `self.ReceivePossessed`
  (params (NewController :type "Controller Object Reference"))
  ;[1 1 1] Input Mappings (change source of setup later)
  (bind _asbp_robot_controller (cast `/Game/Blueprints/BP_RobotController` NewController))
  (bind _returnvalue (pcsubsystem `EnhancedInputLocalPlayerSubsystem` _asbp_robot_controller))
  (`/Engine/EditorBlueprintResources/StandardMacros.IsValid` _returnvalue
    (:`Is Valid`
      (`EnhancedInputSubsystemInterface.AddMappingContext` _returnvalue "/Game/Inputs/IM_Robot.IM_Robot" 0 (struct))
      (`KismetSystemLibrary.PrintString` "Mapping Context Added to Robot"))))

(fn `UserConstructionScript`)