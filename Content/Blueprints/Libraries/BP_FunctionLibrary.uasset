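; Blueprint function library that centralizes shared constants and naming helpers for a level-based game with reflecting lasers.
; Getters supply the laser's maximum length and reflection limit, the highest level number and the default save slot name and user index.
; GetLevelName builds a level name by appending the given number to a "Level" prefix.
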(fn `GetDefaultSaveOptions`
  (returns (`Slot Name` :type String) (`User Index` :type Integer))
  (return "Slot" 0))

(fn `GetLaserMaxLength`
  (returns (Length :type "Float (double-precision)"))
  (return 2000.0))

(fn `GetLevelName`
  (params (Number :type Integer))
  (returns (NewParam :type String))
  (return (`KismetStringLibrary.Concat_StrStr` "Level" (`KismetStringLibrary.Conv_IntToString` Number))))

(fn `GetMaxLevel`
  (returns (Level :type Integer))
  (return 4))

(fn `GetMaxReflections`
  (returns (MaxReflections :type Integer))
  (return 25))