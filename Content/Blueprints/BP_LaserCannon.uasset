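; BP_LaserCannon is a color-coded laser emitter that fires a reflecting beam and tracks the receptor it reaches.
; It spawns a BP_LaserBeam on BeginPlay, sets its color from an ID, and re-shoots along its arrow every Tick.
; Each iteration compares current reflections with the previous set and clears stale ones through their origin mirrors.
; It remembers the last receptor hit and notifies it when the beam stops reaching it.
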(event `self.ReceiveBeginPlay`
  (bind _returnvalue (`|SpawnActorFromClass` "/Game/Blueprints/BP_LaserBeam.BP_LaserBeam_C" (`KismetMathLibrary.MakeTransform` (`SceneComponent.K2_GetComponentLocation` (`self.Arrow`))) "Undefined" "MultiplyWithRoot" null null))
  (set `self.LaserBeam` _returnvalue)
  (switch `/Game/Blueprints/LaserID` (`self.ID`)
    (:`NewEnumerator3`
      (set `self.Color` (struct :`R` 1.0 :`G` 1.0 :`B` 1.0 :`A` 1.0)))
    (:`NewEnumerator0`
      (set `self.Color` (struct :`R` 1.0 :`G` 0.827451 :`A` 1.0)))
    (:`NewEnumerator1`
      (set `self.Color` (struct :`G` 0.300213 :`B` 1.0 :`A` 1.0)))
    (:`NewEnumerator2`
      (set `self.Color` (struct :`R` 1.0 :`G` 0.109804 :`B` 0.839216 :`A` 1.0)))))

(event `self.ReceiveTick`
  (params (DeltaSeconds :type "Float (single-precision)"))
  (`self.Shoot` null))

(fn `GetID`
  (returns (ID :type "/Game/Blueprints/LaserID Enum"))
  (return (`self.ID`)))

(fn `ReachedEndOfLaser`
  (params (CurrentReflections :type "Array of /Game/Blueprints/BP_LaserBeam Object Reference") (PreviousReflections :type "Array of /Game/Blueprints/BP_LaserBeam Object Reference"))
  (set `self.CurrentReflections` CurrentReflections)
  (for _array_element PreviousReflections
    (if (`KismetArrayLibrary.Array_Contains` (`self.CurrentReflections`) _array_element)
      (`/Game/Blueprints/BP_MacroLibrary.Print` "Same reflection found" (struct :`R` 0.381738 :`G` 0.404124 :`B` 0.713726 :`A` 1.0))
      (else
        (`/Game/Blueprints/BP_Mirror.ClearReflection` (`/Game/Blueprints/BP_LaserBeam.GetMirrorOrigin` _array_element) _array_element))))
  (set `self.PreviousReflections` (`self.CurrentReflections`))
  (`/Game/Blueprints/BP_MacroLibrary.Print` (`KismetStringLibrary.Concat_StrStr` "Iteraction ended with " (`KismetStringLibrary.Conv_IntToString` (`KismetArrayLibrary.Array_Length` (`self.CurrentReflections`))) " lasers. The previous one had " (`KismetStringLibrary.Conv_IntToString` (`KismetArrayLibrary.Array_Length` PreviousReflections)) " lasers.") (struct :`R` 0.003922 :`G` 0.713726 :`B` 0.113725 :`A` 1.0))
  (return))

(fn `ReceptorNotFound`
  (bind _lasthitreceptor (`self.LastHitReceptor`))
  (if (`KismetSystemLibrary.IsValid` _lasthitreceptor)
    (`/Game/Blueprints/Receptors/BP_LaserReceptor.RegisterCannonNotReachingAnymore` _lasthitreceptor self)
    (set `self.LastHitReceptor` null)))

(fn `Shoot`
  (params (Manager :type "/Game/Blueprints/BP_LaserCannonManager Object Reference"))
  (bind _laserbeam (`self.LaserBeam`))
  (bind _currentreflections (`self.CurrentReflections`))
  (bind _returnvalue (`SceneComponent.K2_GetComponentLocation` (`self.Arrow`)))
  (set `self.Manager` Manager)
  (`/Game/Blueprints/BP_MacroLibrary.Print` (`KismetStringLibrary.Concat_StrStr` "Starting a new interation. Previous had " (`KismetStringLibrary.Conv_IntToString` (`KismetArrayLibrary.Array_Length` (`self.PreviousReflections`))) " lasers.") (`self.Color`))
  (`KismetArrayLibrary.Array_Clear` (`self.CurrentReflections`))
  (`KismetArrayLibrary.Array_AddUnique` _currentreflections _laserbeam)
  (`/Game/Blueprints/BP_LaserBeam.ShootLaser` _laserbeam _returnvalue (+ _returnvalue (* (`KismetMathLibrary.GetForwardVector` (`SceneComponent.K2_GetComponentRotation` (`self.Arrow`))) (`/Game/Blueprints/BPFL_Constants.GetLaserMaxLength`))) (`self.Color`) self (`self.PreviousReflections`) _currentreflections self))

(fn `Successfuly Reached Receptor`
  (params (Receptor :type "/Game/Blueprints/Receptors/BP_LaserReceptor Object Reference"))
  (set `self.LastHitReceptor` Receptor))

(fn `UserConstructionScript`)