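; BP_LaserCannonManager fires the level's laser cannons one after another in a repeating cycle.
; On BeginPlay it collects every BP_LaserCannon actor and starts a looping one-second timer.
; Each tick of the timer calls Shoot on the current cannon, then advances the index and wraps it back to the first.
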(event `self.ReceiveBeginPlay`
  (set `self.Index` 0)
  (bind _outactors (`GameplayStatics.GetAllActorsOfClass` "/Game/Blueprints/BP_LaserCannon.BP_LaserCannon_C"))
  (set `self.Cannons` _outactors)
  (`KismetSystemLibrary.K2_SetTimer` null "ShootNextCannon" 1.0 true))

(fn `ShootNextCannon`
  (`/Game/Blueprints/BP_LaserCannon.Shoot` (`|GetArrayItem` (`self.Cannons`) (`self.Index`)) self)
  (`/Engine/EditorBlueprintResources/StandardMacros.IncrementInt` (`self.Index`)
    (:`  `
      (if (>= (`self.Index`) (`KismetArrayLibrary.Array_Length` (`self.Cannons`)))
        (set `self.Index` 0)))))

(fn `UserConstructionScript`)